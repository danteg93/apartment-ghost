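; AI character that reacts to nearby ToggleDoors opening or closing by moving away.
; On BeginPlay it subscribes to every door's AI enter/exit radius dispatchers and binds doors it already overlaps.
; Entering a radius binds that door's open and close events, and exiting unbinds them.
; Either event triggers a temporary RunAway, a simple move to a hard-coded point; some older binding logic is left unconnected.
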(event `Check overlapping actors`
  (params (Door :type "/Game/Blueprints/ToggleDoor Object Reference"))
  ;[1 1 1] Bind Enter radius event
)

(event `self.ReceiveBeginPlay`
  ;[0 1 0.8092] Listen for all ToggleDoor's AI interaction radius messages.
  (bind _outactors (`GameplayStatics.GetAllActorsOfClass` "/Game/Blueprints/ToggleDoor.ToggleDoor_C"))
  (for _array_element _outactors
    (add `/Game/Blueprints/ToggleDoor.AI Enter Radius` _array_element (delegate `CallBindToggleDoor`))
    (add `/Game/Blueprints/ToggleDoor.AI Exit Radius` _array_element (delegate `CallUnbindToggleDoor`)))
  ;[0 0.38 1] Bind already overlapping ToggleDoor's open / close events on game start.
  (for _array_element_2 (`self.GetOverlappingActors` self "/Game/Blueprints/ToggleDoor.ToggleDoor_C")
    (bind _astoggle_door (cast `/Game/Blueprints/ToggleDoor` _array_element_2))
    (`self.BindToggleDoor` _astoggle_door)))

(event `CallBindToggleDoor`
  (params (Door :type "/Game/Blueprints/ToggleDoor Object Reference"))
  ;[0 1 0.8092] Listen for all ToggleDoor's AI interaction radius messages.
  (`self.BindToggleDoor` Door))

(event `CallUnbindToggleDoor`
  (params (Door :type "/Game/Blueprints/ToggleDoor Object Reference"))
  ;[0 1 0.8092] Listen for all ToggleDoor's AI interaction radius messages.
  (`self.UnbindToggleDoor` Door))

(event `BindToggleDoor`
  (params (Door :type "/Game/Blueprints/ToggleDoor Object Reference"))
  ;[0 1 0.08367] Helpful Bind / Unbind functions for ToggleDoors
  (add `/Game/Blueprints/ToggleDoor.DoorOpen` Door (delegate `CallRunAway`))
  (add `/Game/Blueprints/ToggleDoor.DoorClose` Door (delegate `CallRunAway`)))

(event `RunAway`
  ;[1 0.05867 0.1064] Run to some Fixed point when door opens/closes (Temporary)
  (`NavigationSystem.SimpleMoveToLocation` (`self.GetController` self) (`KismetMathLibrary.MakeVector` 400.0 400.0 20.0)))

(event `CallRunAway`
  (params (DoorLoc :type "Vector Structure"))
  ;[0 1 0.08367] Helpful Bind / Unbind functions for ToggleDoors
  (`self.RunAway`))

(event `UnbindToggleDoor`
  (params (Door :type "/Game/Blueprints/ToggleDoor Object Reference"))
  ;[0 1 0.08367] Helpful Bind / Unbind functions for ToggleDoors
  (remove `/Game/Blueprints/ToggleDoor.DoorOpen` Door (delegate `CallRunAway`))
  (remove `/Game/Blueprints/ToggleDoor.DoorClose` Door (delegate `CallRunAway`)))

(fn `UserConstructionScript`)