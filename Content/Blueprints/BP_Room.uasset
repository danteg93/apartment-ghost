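; BP_Room is a room that tracks its own scare level as AI characters get scared.
; On BeginPlay it finds every AI_Character and binds to the AIScared event on each one's Scarable_AI controller, reached through the character's Instigator.
; Each event passes the room where the scare happened, and the room raises its ScareLevel by a fixed step only when that room is itself.
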(event `self.ReceiveBeginPlay`
  (bind _outactors (`GameplayStatics.GetAllActorsOfClass` "/Game/Blueprints/AI/AI_Character.AI_Character_C"))
  (for _array_element _outactors
    (bind _asscarable_ai (cast `/Game/Blueprints/AI/Scarable_AI/Scarable_AI` (`Pawn.GetController` (`Actor.Instigator` _array_element))))
    (add `/Game/Blueprints/AI/Scarable_AI/Scarable_AI.AI Scared` _asscarable_ai (delegate `Increase Scare Level`))))

(event `Increase Scare Level`
  (params (`Scared Room` :type "/Game/Blueprints/BP_Room Object Reference"))
  (if (== `Scared Room` self)
    (set `self.ScareLevel` (+ 5 (`self.ScareLevel`)))))

(fn `UserConstructionScript`)