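; Interactable bed that shakes when touched and fires a scare event, ignoring touches while already shaking.
; A ShakeBed timeline bobs the SimpleBed component vertically around the location cached at construction and wobbles its rotation from the value captured on touch.
; Yaw reuses the pitch curve and initial pitch, and the captured world rotation is applied as relative.
; When the timeline finishes, it clears the shaking and interaction flags.
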(event `self.ReceiveActorOnInputTouchBegin`
  (params (FingerIndex :type "ETouchIndex Enum" :default "Touch1"))
  (bind (_initialposition_x _initialposition_y _initialposition_z) (`KismetMathLibrary.BreakVector` (`self.InitialPosition`)))
  (bind (_initialrotation_roll _initialrotation_pitch) (`KismetMathLibrary.BreakRotator` (`self.initialRotation`)))
  ;[0.1031 0.1158 1] If object is shaking then do nothing, else start animation
  (if (not (`self.isShaking`))
    (set `self.isShaking` true)
    (`self.Scare Event` self)
    (set `self.initialRotation` (`SceneComponent.K2_GetComponentRotation` (`self.Simple Bed`)))
    ;[0.1378 0.485 0] Animation for Shake, when finished change shaking flag
    (bind (_direction _rotationbedx _rotationbedy _positionbedz) (`Timeline|ShakeBed` :!via `PlayFromStart`)
      (:`Update`
        (`SceneComponent.K2_SetWorldLocation` (`self.Simple Bed`) (`KismetMathLibrary.MakeVector` _initialposition_x _initialposition_y (+ _initialposition_z (* _positionbedz 20.0))) false false)
        (bind _returnvalue (+ (* 10.0 _rotationbedy) _initialrotation_pitch))
        (`SceneComponent.K2_SetRelativeRotation` (`self.Simple Bed`) (`KismetMathLibrary.MakeRotator` (+ (* _rotationbedx 10.0) _initialrotation_roll) _returnvalue _returnvalue) false false))
      (:`Finished`
        (set `self.isShaking` false)
        (set `self.IsBeingInteractedWith` false)))))

(fn `UserConstructionScript`
  (set `self.InitialPosition` (`SceneComponent.K2_GetComponentLocation` (`self.Simple Bed`)))
  (set `self.isShaking` false))