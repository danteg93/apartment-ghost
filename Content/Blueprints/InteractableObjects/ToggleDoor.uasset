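; Interactable door actor that the player toggles by click or touch, swinging it open or closed with sound and optionally starting open.
; A timeline adds yaw to the rotation cached at construction, playing forward to open and in reverse to close.
; Event dispatchers broadcast each toggle with the door's location.
; Two trigger volumes also dispatch events when AI characters enter or leave awareness and interaction range.
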(event `Open Door`
  (bind (_init_rotation_roll _init_rotation_pitch _init_rotation_yaw) (`KismetMathLibrary.BreakRotator` (`self.Init Rotation`)))
  ;[0 1 0.02078] Calculate new rotation and apply the animation to the door actor.
  (`GameplayStatics.PlaySoundAtLocation` "/Game/SoundEffects/DOOR-OPEN.DOOR-OPEN" (`self.K2_GetActorLocation`))
  (bind (_direction _door_rotation) (`Timeline|Door Movement` :!via `PlayFromStart` :!label _label)
    (:`Update`
      (`self.K2_SetActorRelativeRotation` (`KismetMathLibrary.MakeRotator` _init_rotation_roll _init_rotation_pitch (+ _door_rotation _init_rotation_yaw))))))

(event `Close Door`
  ;[0 1 0.02078] Calculate new rotation and apply the animation to the door actor.
  (`GameplayStatics.PlaySoundAtLocation` "/Game/SoundEffects/DOOR-CLOSE.DOOR-CLOSE" (`self.K2_GetActorLocation`))
  (goto _label :!via `ReverseFromEnd`))

(event `self.ReceiveBeginPlay`
  (bind (_init_rotation_roll _init_rotation_pitch _init_rotation_yaw) (`KismetMathLibrary.BreakRotator` (`self.Init Rotation`)))
  ;[0.9609 0.1681 1] Rotate door 90 degrees if it is open by default.
  (if (`self.isOpen`)
    (`self.SetActorRotation` (`KismetMathLibrary.MakeRotator` _init_rotation_roll _init_rotation_pitch (+ 90.0 _init_rotation_yaw)))))

(event `self.Door.OnInputTouchBegin`
  (params (FingerIndex :type "ETouchIndex Enum" :default "Touch1") (TouchedComponent :type "PrimitiveComponent Object Reference"))
  (bind _returnvalue (`self.K2_GetActorLocation`))
  (if (`self.isOpen`) :!label _label_2
    (set `self.isOpen` false)
    ;[0 1 0.9558] Dispatch events for opening / closing doors so other Blueprints are aware.
    (`self.Door Close` _returnvalue)
    (`self.Close Door`)
    (else
      (set `self.isOpen` true)
      (`self.Door Open` _returnvalue)
      (`self.Open Door`))))

(event `self.Door.OnClicked`
  (params (TouchedComponent :type "PrimitiveComponent Object Reference"))
  (goto _label_2))

(event `self.AI Interaction Radius.OnComponentBeginOverlap`
  (params (OtherActor :type "Actor Object Reference") (OtherComp :type "PrimitiveComponent Object Reference") (OtherBodyIndex :type Integer) (bFromSweep :type Boolean) (SweepResult :type "HitResult Structure (by ref)"))
  ;[1 0.9385 0] Fire enter and exit events when AI come close enough to interact with the door.
  (if (== (`GameplayStatics.GetObjectClass` OtherActor) "/Game/Blueprints/AI_Character.AI_Character_C")
    (`self.AI Enter Radius` self)))

(event `self.AI Interaction Radius.OnComponentEndOverlap`
  (params (OtherActor :type "Actor Object Reference") (OtherComp :type "PrimitiveComponent Object Reference") (OtherBodyIndex :type Integer))
  ;[1 0.9385 0] Fire enter and exit events when AI come close enough to interact with the door.
  (if (== (`GameplayStatics.GetObjectClass` OtherActor) "/Game/Blueprints/AI_Character.AI_Character_C")
    (`self.AI Exit Radius` self)))

(event `self.Interactable Radius.OnComponentBeginOverlap`
  (params (OtherActor :type "Actor Object Reference") (OtherComp :type "PrimitiveComponent Object Reference") (OtherBodyIndex :type Integer) (bFromSweep :type Boolean) (SweepResult :type "HitResult Structure (by ref)"))
  ;[1 0.4053 0] Fire enter and exit events when the AI is close enough to open / close the door.
  (if (== (`GameplayStatics.GetObjectClass` OtherActor) "/Game/Blueprints/AI_Character.AI_Character_C")
    (`self.Door Interactable` self)))

(event `self.Interactable Radius.OnComponentEndOverlap`
  (params (OtherActor :type "Actor Object Reference") (OtherComp :type "PrimitiveComponent Object Reference") (OtherBodyIndex :type Integer))
  ;[1 0.4053 0] Fire enter and exit events when the AI is close enough to open / close the door.
  (if (== (`GameplayStatics.GetObjectClass` OtherActor) "/Game/Blueprints/AI_Character.AI_Character_C")
    (`self.Door Uninteractable` self)))

(fn `UserConstructionScript`
  (bind _returnvalue (`self.K2_GetActorRotation`))
  (`self.SetActorRotation` _returnvalue)
  (set `self.Init Rotation` _returnvalue))