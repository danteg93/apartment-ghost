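; Interactable door that toggles open and closed on touch, with a sound for each direction.
; A DoorAnimation timeline, played forward or reversed, drives yaw relative to the rotation cached in the construction script, flagging IsBeingInteractedWith until finished.
; Doors marked open by default start rotated 90 degrees on BeginPlay.
; The actor also registers as a sight stimuli source for AI perception.
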(event `self.ReceiveBeginPlay`
  (bind (_init_rotation_roll _init_rotation_pitch _init_rotation_yaw) (`KismetMathLibrary.BreakRotator` (`self.Init Rotation`)))
  (`AIPerceptionSystem.RegisterPerceptionStimuliSource` "/Script/AIModule.AISense_Sight" self)
  ;[0.9609 0.1681 1] Rotate door 90 degrees if it is open by default.
  (if (`self.isOpen`)
    (`self.SetActorRotation` (`KismetMathLibrary.MakeRotator` _init_rotation_roll _init_rotation_pitch (+ 90.0 _init_rotation_yaw)))))

(event `self.Door.OnInputTouchBegin`
  (params (FingerIndex :type "ETouchIndex Enum" :default "Touch1") (TouchedComponent :type "PrimitiveComponent Object Reference"))
  (bind _returnvalue (`self.K2_GetActorLocation`))
  (bind (_init_rotation_roll _init_rotation_pitch _init_rotation_yaw) (`KismetMathLibrary.BreakRotator` (`self.Init Rotation`)))
  (set `self.IsBeingInteractedWith` true)
  (if (`self.isOpen`)
    (set `self.isOpen` false)
    (`GameplayStatics.PlaySoundAtLocation` "/Game/SoundEffects/DOOR-CLOSE.DOOR-CLOSE" _returnvalue)
    (bind (_direction _door_animation) (`Timeline|Door Animation` :!via `ReverseFromEnd` :!label _label)
      (:`Update`
        (`self.K2_SetActorRelativeRotation` (`KismetMathLibrary.MakeRotator` _init_rotation_roll _init_rotation_pitch (+ _door_animation _init_rotation_yaw))))
      (:`Finished`
        (set `self.IsBeingInteractedWith` false)))
    (else
      (set `self.isOpen` true)
      (`GameplayStatics.PlaySoundAtLocation` "/Game/SoundEffects/DOOR-OPEN.DOOR-OPEN" _returnvalue)
      (goto _label :!via `PlayFromStart`))))

(fn `UserConstructionScript`
  (bind _returnvalue (`self.K2_GetActorRotation`))
  (`self.SetActorRotation` _returnvalue)
  (set `self.Init Rotation` _returnvalue))