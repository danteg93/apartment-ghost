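; ToggleLight is an interactable light actor that switches its main light on and off and reports changes through event dispatchers.
; ToggleLight flips MainLight visibility, then broadcasts LightOn or LightOff with the actor's location.
; An interaction radius broadcasts AIEnterRadius and AIExitRadius on overlap, intended for nearby AI.
; The enter check compares the overlapping actor's class to ToggleLightButton, while the exit check's class is left unset.
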(event `Toggle Light`
  (bind _returnvalue (`self.K2_GetActorLocation`))
  (bind _mainlight (`self.MainLight`))
  (`SceneComponent.ToggleVisibility` _mainlight false)
  ;[0 1 0.9659] Dispatch events for turning on / off lights.
  (if (`SceneComponent.IsVisible` _mainlight)
    (`self.LightOn` _returnvalue)
    (else
      (`self.LightOff` _returnvalue))))

(event `self.AI Interaction Radius.OnComponentBeginOverlap`
  (params (OtherActor :type "Actor Object Reference") (OtherComp :type "PrimitiveComponent Object Reference") (OtherBodyIndex :type Integer) (bFromSweep :type Boolean) (SweepResult :type "HitResult Structure (by ref)"))
  ;[1 0.9436 0.04036] Fire enter and exit events when AI come close enough  to interact with the light.
  (if (== (`GameplayStatics.GetObjectClass` OtherActor) "/Game/Blueprints/ToggleLightButton.ToggleLightButton_C")
    (`self.AI Enter Radius` self)))

(event `self.AI Interaction Radius.OnComponentEndOverlap`
  (params (OtherActor :type "Actor Object Reference") (OtherComp :type "PrimitiveComponent Object Reference") (OtherBodyIndex :type Integer))
  ;[1 0.9436 0.04036] Fire enter and exit events when AI come close enough  to interact with the light.
  (if (== (`GameplayStatics.GetObjectClass` OtherActor) null)
    (`self.AI Exit Radius` null)))

(fn `UserConstructionScript`)