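; Interactable bed that shakes when touched, ignoring further touches until the shake finishes.
; A touch broadcasts the bed's initial position, then the ShakeBed timeline offsets the cube's height and rotation from stored starting values.
; An AI interaction radius broadcasts enter and exit events with the bed as payload, only for overlapping actors of class ToggleLightButton.
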(event `Dispatch Shake Bed`
  ;[1 1 1] Event Dispatcher
  (`self.BedShaking` (`self.InitialPosition`)))

(event `self.ReceiveActorOnInputTouchBegin`
  (params (FingerIndex :type "ETouchIndex Enum" :default "Touch1"))
  (bind (_initialposition_x _initialposition_y _initialposition_z) (`KismetMathLibrary.BreakVector` (`self.InitialPosition`)))
  (bind (_initialrotation_roll _initialrotation_pitch) (`KismetMathLibrary.BreakRotator` (`self.initialRotation`)))
  ;[0.1031 0.1158 1] If object is shaking then do nothing, else dispatche event and start animation
  (if (not (`self.isShaking`))
    (set `self.isShaking` true)
    (`self.Dispatch Shake Bed`)
    (set `self.initialRotation` (`SceneComponent.K2_GetComponentRotation` (`self.Cube`)))
    ;[0.1378 0.485 0] Animation for Shake, when finished change shaking flag
    (bind (_direction _rotationbedx _rotationbedy _positionbedz) (`Timeline|ShakeBed` :!via `PlayFromStart`)
      (:`Update`
        (`SceneComponent.K2_SetWorldLocation` (`self.Cube`) (`KismetMathLibrary.MakeVector` _initialposition_x _initialposition_y (+ _initialposition_z (* _positionbedz 20.0))) false false)
        (bind _returnvalue (+ (* 10.0 _rotationbedy) _initialrotation_pitch))
        (`SceneComponent.K2_SetRelativeRotation` (`self.Cube`) (`KismetMathLibrary.MakeRotator` (+ (* _rotationbedx 10.0) _initialrotation_roll) _returnvalue _returnvalue) false false))
      (:`Finished`
        (set `self.isShaking` false)))))

(event `self.AI Interaction Radius.OnComponentBeginOverlap`
  (params (OtherActor :type "Actor Object Reference") (OtherComp :type "PrimitiveComponent Object Reference") (OtherBodyIndex :type Integer) (bFromSweep :type Boolean) (SweepResult :type "HitResult Structure (by ref)"))
  ;[1 0.8938 0.005968] Fire enter and exit events when AI come close enough to interact with the bed.
  (if (== (`GameplayStatics.GetObjectClass` OtherActor) "/Game/Blueprints/ToggleLightButton.ToggleLightButton_C")
    (`self.AI Enter Radius` self)))

(event `self.AI Interaction Radius.OnComponentEndOverlap`
  (params (OtherActor :type "Actor Object Reference") (OtherComp :type "PrimitiveComponent Object Reference") (OtherBodyIndex :type Integer))
  ;[1 0.8938 0.005968] Fire enter and exit events when AI come close enough to interact with the bed.
  (if (== (`GameplayStatics.GetObjectClass` OtherActor) "/Game/Blueprints/ToggleLightButton.ToggleLightButton_C")
    (`self.AI Exit Radius` self)))

(fn `UserConstructionScript`
  (set `self.InitialPosition` (`SceneComponent.K2_GetComponentLocation` (`self.Cube`)))
  (set `self.isShaking` false))