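; A player-controlled camera rig that pans and zooms, with the mouse cursor shown from BeginPlay.
; MoveForward and MoveRight axes shift the actor along its local X and Y by Movespeed, without sweep or frame-time scaling.
; The mouse wheel zooms by changing the SpringArm length in fixed steps, with no limits.
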(event `self.ReceiveBeginPlay`
  (set `PlayerController.bShowMouseCursor` true (`GameplayStatics.GetPlayerController` 0)))

(event `InputAxis|MoveForward`
  (params (AxisValue :type "Float (single-precision)"))
  (`self.K2_AddActorLocalOffset` (`KismetMathLibrary.MakeVector` (* AxisValue (`self.movespeed`)))))

(event `InputAxis|MoveRight`
  (params (AxisValue :type "Float (single-precision)"))
  (`self.K2_AddActorLocalOffset` (`KismetMathLibrary.MakeVector` 0.0 (* AxisValue (`self.movespeed`)))))

(event `Key|MouseScrollUp`
  (params (Key :type "Key Structure" :default "AnyKey"))
  (bind _springarm (`self.SpringArm`))
  (:`Pressed`
    (set `SpringArmComponent.TargetArmLength` (- (`SpringArmComponent.TargetArmLength` _springarm) 50.0) _springarm)))

(event `Key|MouseScrollDown`
  (params (Key :type "Key Structure" :default "AnyKey"))
  (bind _springarm (`self.SpringArm`))
  (:`Pressed`
    (set `SpringArmComponent.TargetArmLength` (+ (`SpringArmComponent.TargetArmLength` _springarm) 50.0) _springarm)))

(fn `UserConstructionScript`)