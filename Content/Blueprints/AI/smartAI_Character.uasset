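; AI character that runs away when a nearby BP_ToggleDoor opens or closes.
; On BeginPlay it subscribes to every door's AI radius enter/exit events, meant to toggle open/close bindings, and directly binds doors it already overlaps.
; Door open/close events trigger RunAway, a temporary SimpleMoveToLocation between two hard-coded points, chosen by the character's current position.
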(event `self.ReceiveBeginPlay`
  ;[0 1 0.8092] Listen for all ToggleDoor's AI interaction radius messages.
  (bind _outactors (`GameplayStatics.GetAllActorsOfClass` "/Game/Blueprints/InteractableObjects/BP_ToggleDoor.BP_ToggleDoor_C"))
  (for _array_element _outactors
    (add `/Game/Blueprints/InteractableObjects/BP_ToggleDoor.AI Enter Radius` _array_element (delegate `CallBindToggleDoor`))
    (add `/Game/Blueprints/InteractableObjects/BP_ToggleDoor.AI Exit Radius` _array_element (delegate `CallUnbindToggleDoor`)))
  ;[0 0.38 1] Bind already overlapping ToggleDoor's open / close events on game start.
  (for _array_element_2 (`self.GetOverlappingActors` self "/Game/Blueprints/InteractableObjects/BP_ToggleDoor.BP_ToggleDoor_C")
    (bind _asbp_toggle_door (cast `/Game/Blueprints/InteractableObjects/BP_ToggleDoor` _array_element_2))
    (`self.BindToggleDoor` _asbp_toggle_door)))

(event `CallBindToggleDoor`
  (params (`Toggle Door` :type "/Game/Blueprints/InteractableObjects/BP_ToggleDoor Object Reference"))
  ;[0 1 0.8092] Listen for all ToggleDoor's AI interaction radius messages.
  (`self.BindToggleDoor` null))

(event `CallUnbindToggleDoor`
  (params (`Toggle Door` :type "/Game/Blueprints/InteractableObjects/BP_ToggleDoor Object Reference"))
  ;[0 1 0.8092] Listen for all ToggleDoor's AI interaction radius messages.
  (`self.UnbindToggleDoor` null))

(event `BindToggleDoor`
  (params (Door :type "/Game/Blueprints/InteractableObjects/BP_ToggleDoor Object Reference"))
  ;[0 1 0.08367] Helpful Bind / Unbind functions for ToggleDoors
  (add `/Game/Blueprints/InteractableObjects/BP_ToggleDoor.Door Open` Door (delegate `CallRunAway`))
  (add `/Game/Blueprints/InteractableObjects/BP_ToggleDoor.Door Close` Door (delegate `CallRunAway`)))

(event `RunAway`
  ;[1 0.05867 0.1064] Run to some Fixed point when door opens/closes (Temporary)
  (if (== (`self.K2_GetActorLocation`) (`KismetMathLibrary.MakeVector` 364.2204 400.0 122.14999) :`ErrorTolerance` 20.0)
    (`NavigationSystem.SimpleMoveToLocation` (`self.GetController` self) (`KismetMathLibrary.MakeVector` -400.0 400.0 120.0))
    (else
      (`NavigationSystem.SimpleMoveToLocation` (`self.GetController` self) (`KismetMathLibrary.MakeVector` 400.0 400.0 20.0)))))

(event `CallRunAway`
  (params (DoorLoc :type "Vector Structure"))
  ;[0 1 0.08367] Helpful Bind / Unbind functions for ToggleDoors
  (`self.RunAway`))

(event `UnbindToggleDoor`
  (params (Door :type "/Game/Blueprints/InteractableObjects/BP_ToggleDoor Object Reference"))
  ;[0 1 0.08367] Helpful Bind / Unbind functions for ToggleDoors
  (remove `/Game/Blueprints/InteractableObjects/BP_ToggleDoor.Door Open` Door (delegate `CallRunAway`))
  (remove `/Game/Blueprints/InteractableObjects/BP_ToggleDoor.Door Close` Door (delegate `CallRunAway`)))

(fn `UserConstructionScript`)