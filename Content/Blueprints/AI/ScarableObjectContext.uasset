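; EQS query context that supplies a single scare object to environment queries.
; For a querier controlled by Scarable_AI, it returns that controller's FirstScare actor.
; For an EQS testing pawn, it returns the first BP_ScareObject found in the world, so queries can be previewed without the AI controller.
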(fn ProvideSingleActor
  (params (QuerierActor :type Actor%20Object%20Reference))
  (Utilities|Casting|CastToEQSTestingPawn QuerierActor
    (:then
      (bind _outactors (Actor|GetAllActorsOfClass "/Game/Blueprints/InteractableObjects/BP_ScareObject.BP_ScareObject_C"))
      (LocalVariables|SetTempScareObject (Utilities|Array|Get(acopy) _outactors)))
    (:CastFailed
      (bind _returnvalue (AI|GetAIController QuerierActor))
      (if (!= _returnvalue 0)
        (bind _asscarable_ai (Utilities|Casting|CastToScarable_AI _returnvalue)
          (:then
            (bind _output_get (LocalVariables|SetTempScareObject (Variables|/Game/Blueprints/AI/Scarable_AI.Scarable_AI_C|GetFirst%20Scare _asscarable_ai))))
          (:CastFailed
            _)))))
  (return _output_get))