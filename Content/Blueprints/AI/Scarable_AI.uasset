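; AI controller for scarable characters that react to scare objects being interacted with.
; It runs the Scarable_BT behavior tree on BeginPlay.
; Perception updates pick out BP_ScareObject actors currently being interacted with and pass them to ScareAI.
; ScareAI stores any scare differing from the stored one as FirstScare and writes it to the Blackboard, so despite its name it can be replaced.
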(event `self.ReceiveBeginPlay`
  (`self.RunBehaviorTree` "/Game/Blueprints/AI/Scarable_BT.Scarable_BT"))

(event `self.AIPerception.OnPerceptionUpdated`
  (params (UpdatedActors :type "Array of Actor Object Reference"))
  (for _array_element UpdatedActors
    (bind _asbp_scare_object (cast `/Game/Blueprints/InteractableObjects/BP_ScareObject` _array_element))
    (if (`/Game/Blueprints/InteractableObjects/BP_ScareObject.IsBeingInteractedWith` _asbp_scare_object)
      (`self.Scare AI` _asbp_scare_object))))

(fn `Scare AI`
  (params (`New Scare` :type "Actor Object Reference"))
  (if (!= `New Scare` (`self.First Scare`))
    (bind _output_get (set `self.First Scare` `New Scare`))
    (`BlackboardComponent.SetValueAsObject` (`AIBlueprintHelperLibrary.GetBlackboard` null) (`self.BlackboardKeyFirstScare`) _output_get)))

(fn `UserConstructionScript`)